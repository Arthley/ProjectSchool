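; Player-controlled Star Destroyer that constantly moves along its forward vector at a stepped throttle speed.
; Enhanced Input speed-up/down actions shift a target index into the Speeds array.
; Tick walks the current index toward that target one step at a time, lerping speed over per-step acceleration or deceleration durations.
; When target matches current, speed eases back using the last transition's elapsed time; Tick also prints speed for debugging.
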(event `self.ReceiveBeginPlay`
  ;[0.8871 0.5121 1] On begin Play
  (bind _asplayer_controller (cast `PlayerController` (`self.GetController`)))
  (`/Engine/EditorBlueprintResources/StandardMacros.IsValid` _asplayer_controller
    (:`Is Valid`
      (`EnhancedInputSubsystemInterface.AddMappingContext` (pcsubsystem `EnhancedInputLocalPlayerSubsystem` _asplayer_controller) "/Game/Core/Blueprint/Input/IMC_Spaceship.IMC_Spaceship" 0 (struct))
      (set `PlayerController.bShowMouseCursor` true (`GameplayStatics.GetPlayerController` 0))
      (bind _output_get (set `self.State Index` 1))
      (set `self.Current State Index` _output_get))))

(event `self.ReceiveTick`
  (params (DeltaSeconds :type "Float (single-precision)"))
  (bind _output (`|GetArrayItem` (`self.Speeds`) (`self.Current State Index`)))
  (bind _output_2 (`|GetArrayItem` (`self.Speeds`) (+ 1 (`self.Current State Index`))))
  (bind _output_3 (`|GetArrayItem` (`self.Speeds`) (- (`self.Current State Index`) 1)))
  ;[1 0.383 0.5032] Movement by step
  (`self.K2_AddActorWorldOffset` (* DeltaSeconds (* (`KismetMathLibrary.Normal` (`SceneComponent.GetForwardVector` (`self.StarDestroyer`))) (`self.Current Speed`))))
  (`KismetSystemLibrary.PrintString` (`KismetStringLibrary.Conv_DoubleToString` (`self.Current Speed`)))
  (if (== (`self.State Index`) (`self.Current State Index`))
    (if (or (`self.Is Speeding Up`) (`self.Is Speeding Down`))
      (set `self.Current Duration` 0.0)
      (set `self.Is Speeding Up` false)
      (set `self.Is Speeding Down` false))
    (set `self.Initial Speed` (`self.Current Speed`))
    (`self.TimerCurrentDuration`)
    (bind _returnvalue (`self.SetSpeed` (`KismetMathLibrary.Lerp` (`self.Initial Speed`) _output (/ (`self.Current Duration`) (`self.Inverse Duration`))) _output))
    (if _returnvalue
      (`self.ResetParametersafterAcceleration` :!label _label))
    (else
      (if (not (or (`self.Is Speeding Up`) (`self.Is Speeding Down`)))
        (set `self.Current Duration` 0.0))
      (if (> (`self.State Index`) (`self.Current State Index`))
        (set `self.Is Speeding Up` true)
        (`self.TimerCurrentDuration`)
        (`self.InverseDurationCalculation`)
        (bind _returnvalue_2 (`self.SetSpeed` (`KismetMathLibrary.Lerp` (`self.Initial Speed`) _output_2 (/ (`self.Current Duration`) (`|GetArrayItem` (`self.SpeedsUpDuration`) (+ 1 (`self.Current State Index`))))) _output_2))
        (if _returnvalue_2
          (set `self.Current State Index` (+ 1 (`self.Current State Index`)))
          (goto _label))
        (else
          (set `self.Is Speeding Down` true)
          (`self.TimerCurrentDuration`)
          (`self.InverseDurationCalculation`)
          (bind _returnvalue_3 (`self.SetSpeed` (`KismetMathLibrary.Lerp` (`self.Initial Speed`) _output_3 (/ (`self.Current Duration`) (`|GetArrayItem` (`self.SpeedDownDuration`) (- (`self.Current State Index`) 1)))) _output_3))
          (if _returnvalue_3
            (set `self.Current State Index` (- (`self.Current State Index`) 1))
            (goto _label)))))))

(event `EnhancedInput|/Game/Core/Blueprint/Input/IA_SpeedUp`
  (params (ActionValue :type Boolean) (ElapsedSeconds :type "Float (double-precision)") (TriggeredSeconds :type "Float (double-precision)") (InputAction :type "InputAction Object Reference" :default "/Game/Core/Blueprint/Input/IA_SpeedUp.IA_SpeedUp"))
  (bind _state_index (`self.State Index`))
  (bind _returnvalue (- (`KismetArrayLibrary.Array_Length` (`self.Speeds`)) 1))
  ;[1 1 1] Input Speed
  (:`Started`
    (if (!= _state_index _returnvalue)
      (set `self.State Index` (`KismetMathLibrary.Clamp` (+ _state_index 1) 0 _returnvalue)))))

(event `EnhancedInput|/Game/Core/Blueprint/Input/IA_SpeedDown`
  (params (ActionValue :type Boolean) (ElapsedSeconds :type "Float (double-precision)") (TriggeredSeconds :type "Float (double-precision)") (InputAction :type "InputAction Object Reference" :default "/Game/Core/Blueprint/Input/IA_SpeedDown.IA_SpeedDown"))
  (bind _state_index (`self.State Index`))
  ;[1 1 1] Input Speed
  (:`Started`
    (if (!= 0 _state_index)
      (set `self.State Index` (`KismetMathLibrary.Clamp` (- _state_index 1) 0 (- (`KismetArrayLibrary.Array_Length` (`self.Speeds`)) 1))))))

(fn `InverseDurationCalculation`
  (set `self.Inverse Duration` (`self.Current Duration`)))

(fn `ResetParametersafterAcceleration`
  (bind _output_get (set `self.Current Speed` (`|GetArrayItem` (`self.Speeds`) (`self.Current State Index`))))
  (set `self.Initial Speed` _output_get)
  (set `self.Current Duration` 0.0)
  (return))

(fn `SetSpeed`
  (params (`Current Speed` :type "Float (double-precision)") (`Speed by Index` :type "Float (double-precision)"))
  (returns (ReturnValue :type Boolean))
  (set `self.Current Speed` `Current Speed`)
  (return (`KismetMathLibrary.NearlyEqual_FloatFloat` `Current Speed` `Speed by Index` 1.0)))

(fn `TimerCurrentDuration`
  (set `self.Current Duration` (+ (`self.Current Duration`) (`GameplayStatics.GetWorldDeltaSeconds`))))

(fn `UserConstructionScript`)