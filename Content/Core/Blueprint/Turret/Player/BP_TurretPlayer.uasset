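; Player turret, apparently mounted on a Star Destroyer, that fires bullets toward an externally supplied HitLocation.
; Tick draws a debug trace from FireSocket to that point and, while IsFiring, calls FireProjectile through a DoOnce reset after two seconds.
; FireProjectile requires both alignment flags, then spawns BP_BulletPlayer at each turret socket, aimed at HitLocation.
; Bone-aiming logic for yaw and pitch, which also sets those flags, is disconnected and never runs.
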(event `self.ReceiveTick`
  (params (DeltaSeconds :type "Float (single-precision)"))
  (`KismetSystemLibrary.LineTraceSingle` :`Start` (`SceneComponent.GetSocketLocation` (`self.PoseableMesh`) "FireSocket") :`End` (`self.Hit Location`) :`TraceChannel` "TraceTypeQuery3" :`DrawDebugType` "ForDuration" :`TraceColor` (struct :`G` 0.35567 :`B` 1.0 :`A` 1.0) :`DrawTime` 0.0)
  (if (`self.Is Firing`)
    (`/Engine/EditorBlueprintResources/StandardMacros.DoOnce` false :!label _label
      (:`Completed`
        (`self.Fire Projectile`)
        (`KismetSystemLibrary.Delay` 2.0)
        (goto _label :!via `Reset`)))))

(fn `Fire Projectile`
  (if (and (`self.Is Alligned Horizontally`) (`self.Is Alligned Vertically`))
    (bind _returnvalue (`PoseableMeshComponent.GetBoneRotationByName` (`self.PoseableMesh`) (`self.Turret Bone Yaw`) "WorldSpace"))
    (for _array_element (`self.Turret Sockets`)
      (bind _returnvalue_2 (`SceneComponent.GetSocketLocation` (`self.PoseableMesh`) _array_element))
      (bind _returnvalue_3 (`|SpawnActorFromClass` "/Game/Core/Blueprint/Bullet/Player/BP_BulletPlayer.BP_BulletPlayer_C" (`KismetMathLibrary.MakeTransform` _returnvalue_2 _returnvalue) "AdjustIfPossibleButAlwaysSpawn" "MultiplyWithRoot" null null))
      (set `/Game/Core/Blueprint/Bullet/BP_BulletBase.Speed` 60.0 _returnvalue_3)
      (set `/Game/Core/Blueprint/Bullet/BP_BulletBase.Direction` (- (`self.Hit Location`) _returnvalue_2) _returnvalue_3)
      (`/Game/Core/Blueprint/Bullet/BP_BulletBase.Set Bullet Direction` _returnvalue_3))))

(fn `UserConstructionScript`)