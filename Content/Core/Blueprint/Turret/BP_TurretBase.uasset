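; BP_TurretBase is a turret base actor Blueprint containing an unfinished Set Bullet Direction function and an empty construction script.
; The function normalizes a vector, scales its Z, adds a random spread term, prints debug values and offsets the actor itself.
; The source vector, spread amount and final multiplier are all zero, so the offset resolves to zero.
; A random-chance branch sits unexecuted.
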(fn `Set Bullet Direction`
  (bind (_returnvalue_x _returnvalue_y _returnvalue_z) (`KismetMathLibrary.BreakVector` (`KismetMathLibrary.Normal` (0.0 0.0 0.0))))
  (bind _returnvalue (* _returnvalue_z 1000.0))
  (bind _returnvalue_2 (+ (* (+ (* (`KismetMathLibrary.RandomFloat`) 2.0) -1.0) 0.0) _returnvalue))
  (`KismetSystemLibrary.PrintString` (`KismetStringLibrary.Conv_DoubleToString` _returnvalue))
  (`KismetSystemLibrary.PrintString` (`KismetStringLibrary.Conv_DoubleToString` _returnvalue_2))
  (`self.K2_AddActorWorldOffset` (* (`KismetMathLibrary.MakeVector` _returnvalue_x _returnvalue_y _returnvalue_2) (0.0 0.0 0.0))))

(fn `UserConstructionScript`)