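; Player-controlled Star Destroyer spaceship with throttle steps, strafing, rotation and turret fire, driven by Enhanced Input.
; Tick offsets the actor using forward speed lerped between indexed steps plus accelerating/decaying vertical and lateral speeds, and applies ACRotator's rotation to the AndorianCruiser component.
; A mode toggle gates translation versus turn/roll input.
; A camera-through-spring-arm trace supplies the aim point to child BP_Turrets, while the HUD shows current and target speed.
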(event `self.ReceiveBeginPlay`
  ;[0.8871 0.5121 1] On begin Play
  (bind _asplayer_controller (cast `PlayerController` (`self.GetController`)))
  (`/Engine/EditorBlueprintResources/StandardMacros.IsValid` _asplayer_controller
    (:`Is Valid`
      (`EnhancedInputSubsystemInterface.AddMappingContext` (pcsubsystem `EnhancedInputLocalPlayerSubsystem` _asplayer_controller) "/Game/Core/Blueprint/Input/IMC_Spaceship.IMC_Spaceship" 0 (struct))
      (bind _output_get (set `self.State Index` 1))
      (set `self.Current State Index` _output_get)
      (`self.Add Turret`)
      (bind _returnvalue (`|CreateWidget` "/Game/Core/Blueprint/Widget/WB_HUD_Core.WB_HUD_Core_C" (`GameplayStatics.GetPlayerController` 0)))
      (bind _output_get_2 (set `self.HUD Core` _returnvalue))
      (`UserWidget.AddToViewport` _output_get_2 0))))

(event `self.ReceiveTick`
  (params (DeltaSeconds :type "Float (single-precision)"))
  ;[1 0.383 0.5032] Movement by step
  (bind _finalspeed (`self.CalculateSpeed` DeltaSeconds))
  (`self.K2_AddActorWorldOffset` _finalspeed)
  (`SceneComponent.K2_AddLocalRotation` (`self.Andorian Cruiser`) (`/Game/Core/Blueprint/AC/AC_Rotator.Final Rotator` (`self.AC_Rotator`)) false false)
  (`self.SMHorizontalSpeed`)
  (`self.SMVerticalSpeed`)
  (`self.SMLateralSpeed`)
  (`self.Calculate Distance from Target`)
  (for _array_element (`self.Turrets`)
    (set `/Game/Core/Blueprint/Player/BP_Turret.Hit Location` (`self.Main Hit Location`) _array_element)))

(event `EnhancedInput|/Game/Core/Blueprint/Input/IA_SpeedUp`
  (params (ActionValue :type Boolean) (ElapsedSeconds :type "Float (double-precision)") (TriggeredSeconds :type "Float (double-precision)") (InputAction :type "InputAction Object Reference" :default "/Game/Core/Blueprint/Input/IA_SpeedUp.IA_SpeedUp"))
  (bind _state_index (`self.State Index`))
  (bind _returnvalue (- (`KismetArrayLibrary.Array_Length` (`self.Speeds`)) 1))
  ;[1 1 1] Input
  (:`Started`
    (if (!= _state_index _returnvalue)
      (set `self.State Index` (`KismetMathLibrary.Clamp` (+ _state_index 1) 0 _returnvalue)))))

(event `EnhancedInput|/Game/Core/Blueprint/Input/IA_TurnLeft`
  (params (ActionValue :type Boolean) (ElapsedSeconds :type "Float (double-precision)") (TriggeredSeconds :type "Float (double-precision)") (InputAction :type "InputAction Object Reference" :default "/Game/Core/Blueprint/Input/IA_TurnLeft.IA_TurnLeft"))
  (bind _ac_rotator (`self.AC_Rotator`))
  ;[1 1 1] Input
  (:`Triggered`
    (if (`self.Is Rotating Mode`)
      (if (not (`/Game/Core/Blueprint/AC/AC_Rotator.Is Turning Right` _ac_rotator))
        (set `/Game/Core/Blueprint/AC/AC_Rotator.Is Turning Left` true _ac_rotator))))
  (:`Completed`
    (set `/Game/Core/Blueprint/AC/AC_Rotator.Is Turning Left` false _ac_rotator)))

(event `EnhancedInput|/Game/Core/Blueprint/Input/IA_MoveLeft`
  (params (ActionValue :type Boolean) (ElapsedSeconds :type "Float (double-precision)") (TriggeredSeconds :type "Float (double-precision)") (InputAction :type "InputAction Object Reference" :default "/Game/Core/Blueprint/Input/IA_MoveLeft.IA_MoveLeft"))
  ;[1 1 1] Input
  (:`Triggered`
    (if (`self.Is Rotating Mode`)
      _
      (elif (not (`self.Is Moving Right`))
        (set `self.Is Moving Left` true))))
  (:`Completed`
    (set `self.Is Moving Left` false)))

(event `EnhancedInput|/Game/Core/Blueprint/Input/IA_TurnRight`
  (params (ActionValue :type Boolean) (ElapsedSeconds :type "Float (double-precision)") (TriggeredSeconds :type "Float (double-precision)") (InputAction :type "InputAction Object Reference" :default "/Game/Core/Blueprint/Input/IA_TurnRight.IA_TurnRight"))
  (bind _ac_rotator (`self.AC_Rotator`))
  ;[1 1 1] Input
  (:`Triggered`
    (if (`self.Is Rotating Mode`)
      (if (not (`/Game/Core/Blueprint/AC/AC_Rotator.Is Turning Left` _ac_rotator))
        (set `/Game/Core/Blueprint/AC/AC_Rotator.Is Turning Right` true _ac_rotator))))
  (:`Completed`
    (set `/Game/Core/Blueprint/AC/AC_Rotator.Is Turning Right` false _ac_rotator)))

(event `EnhancedInput|/Game/Core/Blueprint/Input/IA_MoveRight`
  (params (ActionValue :type Boolean) (ElapsedSeconds :type "Float (double-precision)") (TriggeredSeconds :type "Float (double-precision)") (InputAction :type "InputAction Object Reference" :default "/Game/Core/Blueprint/Input/IA_MoveRight.IA_MoveRight"))
  ;[1 1 1] Input
  (:`Triggered`
    (if (`self.Is Rotating Mode`)
      _
      (elif (not (`self.Is Moving Left`))
        (set `self.Is Moving Right` true))))
  (:`Completed`
    (set `self.Is Moving Right` false)))

(event `EnhancedInput|/Game/Core/Blueprint/Input/IA_SpeedDown`
  (params (ActionValue :type Boolean) (ElapsedSeconds :type "Float (double-precision)") (TriggeredSeconds :type "Float (double-precision)") (InputAction :type "InputAction Object Reference" :default "/Game/Core/Blueprint/Input/IA_SpeedDown.IA_SpeedDown"))
  (bind _state_index (`self.State Index`))
  ;[1 1 1] Input
  (:`Started`
    (if (!= 0 _state_index)
      (set `self.State Index` (`KismetMathLibrary.Clamp` (- _state_index 1) 0 (- (`KismetArrayLibrary.Array_Length` (`self.Speeds`)) 1))))))

(event `EnhancedInput|/Game/Core/Blueprint/Input/IA_TurnUp`
  (params (ActionValue :type Boolean) (ElapsedSeconds :type "Float (double-precision)") (TriggeredSeconds :type "Float (double-precision)") (InputAction :type "InputAction Object Reference" :default "/Game/Core/Blueprint/Input/IA_TurnUp.IA_TurnUp"))
  (bind _ac_rotator (`self.AC_Rotator`))
  ;[1 1 1] Input
  (:`Triggered`
    (if (`self.Is Rotating Mode`)
      (if (not (`/Game/Core/Blueprint/AC/AC_Rotator.Is Turning Down` _ac_rotator))
        (set `/Game/Core/Blueprint/AC/AC_Rotator.Is Turning Up` true _ac_rotator))))
  (:`Completed`
    (set `/Game/Core/Blueprint/AC/AC_Rotator.Is Turning Up` false _ac_rotator)))

(event `EnhancedInput|/Game/Core/Blueprint/Input/IA_MoveUp`
  (params (ActionValue :type Boolean) (ElapsedSeconds :type "Float (double-precision)") (TriggeredSeconds :type "Float (double-precision)") (InputAction :type "InputAction Object Reference" :default "/Game/Core/Blueprint/Input/IA_MoveUp.IA_MoveUp"))
  ;[1 1 1] Input
  (:`Triggered`
    (if (`self.Is Rotating Mode`)
      _
      (elif (not (`self.Is Moving Down`))
        (set `self.Is Moving Up` true))))
  (:`Completed`
    (set `self.Is Moving Up` false)))

(event `EnhancedInput|/Game/Core/Blueprint/Input/IA_TurnDown`
  (params (ActionValue :type Boolean) (ElapsedSeconds :type "Float (double-precision)") (TriggeredSeconds :type "Float (double-precision)") (InputAction :type "InputAction Object Reference" :default "/Game/Core/Blueprint/Input/IA_TurnDown.IA_TurnDown"))
  (bind _ac_rotator (`self.AC_Rotator`))
  ;[1 1 1] Input
  (:`Triggered`
    (if (`self.Is Rotating Mode`)
      (if (not (`/Game/Core/Blueprint/AC/AC_Rotator.Is Turning Up` _ac_rotator))
        (set `/Game/Core/Blueprint/AC/AC_Rotator.Is Turning Down` true _ac_rotator))))
  (:`Completed`
    (set `/Game/Core/Blueprint/AC/AC_Rotator.Is Turning Down` false _ac_rotator)))

(event `EnhancedInput|/Game/Core/Blueprint/Input/IA_MoveDown`
  (params (ActionValue :type Boolean) (ElapsedSeconds :type "Float (double-precision)") (TriggeredSeconds :type "Float (double-precision)") (InputAction :type "InputAction Object Reference" :default "/Game/Core/Blueprint/Input/IA_MoveDown.IA_MoveDown"))
  ;[1 1 1] Input
  (:`Triggered`
    (if (`self.Is Rotating Mode`)
      _
      (elif (not (`self.Is Moving Up`))
        (set `self.Is Moving Down` true))))
  (:`Completed`
    (set `self.Is Moving Down` false)))

(event `EnhancedInput|/Game/Core/Blueprint/Input/IA_Direction`
  (params (ActionValue :type "Vector2D Structure") (ElapsedSeconds :type "Float (double-precision)") (TriggeredSeconds :type "Float (double-precision)") (InputAction :type "InputAction Object Reference" :default "/Game/Core/Blueprint/Input/IA_Direction.IA_Direction"))
  ;[1 1 1] Input
  (:`Triggered`
    (`self.AddControllerYawInput` ActionValue_X)
    (`self.AddControllerPitchInput` (* ActionValue_Y -1.0))))

(event `EnhancedInput|/Game/Core/Blueprint/Input/IA_RollLeft`
  (params (ActionValue :type Boolean) (ElapsedSeconds :type "Float (double-precision)") (TriggeredSeconds :type "Float (double-precision)") (InputAction :type "InputAction Object Reference" :default "/Game/Core/Blueprint/Input/IA_RollLeft.IA_RollLeft"))
  (bind _ac_rotator (`self.AC_Rotator`))
  ;[1 1 1] Input
  (:`Triggered`
    (if (`self.Is Rotating Mode`)
      (if (not (`/Game/Core/Blueprint/AC/AC_Rotator.Is Rolling Right` _ac_rotator))
        (set `/Game/Core/Blueprint/AC/AC_Rotator.Is Rolling Left` true _ac_rotator))))
  (:`Completed`
    (set `/Game/Core/Blueprint/AC/AC_Rotator.Is Rolling Left` false _ac_rotator)))

(event `EnhancedInput|/Game/Core/Blueprint/Input/IA_SwitchMode`
  (params (ActionValue :type Boolean) (ElapsedSeconds :type "Float (double-precision)") (TriggeredSeconds :type "Float (double-precision)") (InputAction :type "InputAction Object Reference" :default "/Game/Core/Blueprint/Input/IA_SwitchMode.IA_SwitchMode"))
  ;[1 1 1] Input
  (:`Started`
    (`/Engine/EditorBlueprintResources/StandardMacros.FlipFlop`
      (:`A`
        (`self.Deactivate Rotating Mode`))
      (:`B`
        (`self.Activate Rotating Mode`)))))

(event `EnhancedInput|/Game/Core/Blueprint/Input/IA_RollRight`
  (params (ActionValue :type Boolean) (ElapsedSeconds :type "Float (double-precision)") (TriggeredSeconds :type "Float (double-precision)") (InputAction :type "InputAction Object Reference" :default "/Game/Core/Blueprint/Input/IA_RollRight.IA_RollRight"))
  (bind _ac_rotator (`self.AC_Rotator`))
  ;[1 1 1] Input
  (:`Triggered`
    (if (`self.Is Rotating Mode`)
      (if (not (`/Game/Core/Blueprint/AC/AC_Rotator.Is Rolling Left` _ac_rotator))
        (set `/Game/Core/Blueprint/AC/AC_Rotator.Is Rolling Right` true _ac_rotator))))
  (:`Completed`
    (set `/Game/Core/Blueprint/AC/AC_Rotator.Is Rolling Right` false _ac_rotator)))

(event `EnhancedInput|/Game/Core/Blueprint/Input/IA_Shoot`
  (params (ActionValue :type Boolean) (ElapsedSeconds :type "Float (double-precision)") (TriggeredSeconds :type "Float (double-precision)") (InputAction :type "InputAction Object Reference" :default "/Game/Core/Blueprint/Input/IA_Shoot.IA_Shoot"))
  (bind _turrets (`self.Turrets`))
  ;[1 1 1] Input
  (:`Triggered`
    (for _array_element _turrets
      (set `/Game/Core/Blueprint/Player/BP_Turret.Is Firing` true _array_element)))
  (:`Completed`
    (for _array_element_2 _turrets
      (set `/Game/Core/Blueprint/Player/BP_Turret.Is Firing` false _array_element_2))))

(fn `Activate Rotating Mode`
  (set `self.Is Rotating Mode` true)
  (set `self.Is Moving Up` false)
  (set `self.Is Moving Down` false)
  (set `self.Is Moving Left` false)
  (set `self.Is Moving Right` false))

(fn `Add Turret`
  (for _array_element (`self.GetAllChildActors` true)
    (bind _asbp_turret (cast `/Game/Core/Blueprint/Player/BP_Turret` _array_element))
    (`KismetArrayLibrary.Array_Add` (`self.Turrets`) _asbp_turret)))

(fn `BooleanConverter`
  (params (Boolean :type Boolean))
  (returns (ReturnValue :type "Float (double-precision)"))
  (return (- (* (+ (`KismetMathLibrary.Conv_BoolToDouble` Boolean) 1.0) 2.0) 3.0)))

(fn `Calculate Distance from Target`
  (bind _returnvalue (`SceneComponent.K2_GetComponentLocation` (`self.SpringArm`)))
  (bind (_outhit _returnvalue_2) (`KismetSystemLibrary.LineTraceSingle` :`Start` _returnvalue :`End` (+ _returnvalue (* (`KismetMathLibrary.Normal` (- _returnvalue (`PlayerCameraManager.GetCameraLocation` (`PlayerController.PlayerCameraManager` (`GameplayStatics.GetPlayerController` 0))))) (`self.Target Distance`))) :`TraceChannel` "TraceTypeQuery3" :`DrawDebugType` "ForDuration" :`DrawTime` 1.0))
  (if _returnvalue_2
    (bind (_bblockinghit _binitialoverlap _time _distance _location _impactpoint _normal _impactnormal _physmat _hitactor _hitcomponent _hitbonename _bonename _hititem _elementindex _faceindex _tracestart _traceend) (`GameplayStatics.BreakHitResult` _outhit))
    (set `self.Main Hit Location` _impactpoint)
    (else
      (set `self.Main Hit Location` _traceend)))
  (return))

(fn `CalculateSpeed`
  (params (DeltaSeconds :type "Float (single-precision)"))
  (returns (FinalSpeed :type "Vector Structure"))
  (return (* (+ (* (`KismetMathLibrary.Normal` (`SceneComponent.GetForwardVector` (`self.Andorian Cruiser`))) (`self.Current Speed`)) (* (`KismetMathLibrary.Normal` (`SceneComponent.GetUpVector` (`self.Andorian Cruiser`))) (`self.Current Vertical Speed`)) (* (`KismetMathLibrary.Normal` (`SceneComponent.GetRightVector` (`self.Andorian Cruiser`))) (`self.Current Lateral Speed`))) DeltaSeconds)))

(fn `Deactivate Rotating Mode`
  (bind _ac_rotator (`self.AC_Rotator`))
  (set `self.Is Rotating Mode` false)
  (set `/Game/Core/Blueprint/AC/AC_Rotator.Is Turning Left` false _ac_rotator)
  (set `/Game/Core/Blueprint/AC/AC_Rotator.Is Turning Right` false _ac_rotator)
  (set `/Game/Core/Blueprint/AC/AC_Rotator.Is Turning Down` false _ac_rotator)
  (set `/Game/Core/Blueprint/AC/AC_Rotator.Is Turning Up` false _ac_rotator)
  (set `/Game/Core/Blueprint/AC/AC_Rotator.Is Rolling Left` false _ac_rotator)
  (set `/Game/Core/Blueprint/AC/AC_Rotator.Is Rolling Right` false _ac_rotator))

(fn `InverseDurationCalculation`
  (set `self.Inverse Duration` (`self.Current Duration`)))

(fn `ResetParametersafterAcceleration`
  (bind _output_get (set `self.Current Speed` (`|GetArrayItem` (`self.Speeds`) (`self.Current State Index`))))
  (set `self.Initial Speed` _output_get)
  (set `self.Current Duration` 0.0)
  (return))

(fn `SetSpeed`
  (params (`Current Speed` :type "Float (double-precision)") (`Speed by Index` :type "Float (double-precision)"))
  (returns (ReturnValue :type Boolean))
  (set `self.Current Speed` `Current Speed`)
  (return (`KismetMathLibrary.NearlyEqual_FloatFloat` `Current Speed` `Speed by Index` 1.0)))

(fn `SMHorizontalSpeed`
  (bind _speeds (`self.Speeds`))
  (bind _output (`|GetArrayItem` (`self.Speeds`) (`self.Current State Index`)))
  (bind _output_2 (`|GetArrayItem` (`self.Speeds`) (+ 1 (`self.Current State Index`))))
  (bind _output_3 (`|GetArrayItem` (`self.Speeds`) (- (`self.Current State Index`) 1)))
  (set `/Game/Core/Blueprint/Widget/WB_HUD_Core.TSpeedSlider` (/ (`KismetMathLibrary.Conv_IntToDouble` (`self.State Index`)) 5.0) (`self.HUD Core`))
  (set `/Game/Core/Blueprint/Widget/WB_HUD_Core.CSpeedSlider` (+ (/ (`self.Current Speed`) (- (`|GetArrayItem` _speeds (- (`KismetArrayLibrary.Array_Length` _speeds) 1)) (`|GetArrayItem` _speeds))) 0.2) (`self.HUD Core`))
  (if (== (`self.State Index`) (`self.Current State Index`))
    (if (or (`self.Is Moving Forward`) (`self.Is Moving Backward`))
      (set `self.Current Duration` 0.0)
      (set `self.Is Moving Forward` false)
      (set `self.Is Moving Backward` false))
    (set `self.Initial Speed` (`self.Current Speed`))
    (`self.TimerCurrentDuration`)
    (bind _returnvalue (`self.SetSpeed` (`KismetMathLibrary.Lerp` (`self.Initial Speed`) _output (/ (`self.Current Duration`) (`self.Inverse Duration`))) _output))
    (if _returnvalue
      (`self.ResetParametersafterAcceleration` :!label _label))
    (else
      (if (not (or (`self.Is Moving Forward`) (`self.Is Moving Backward`)))
        (set `self.Current Duration` 0.0))
      (if (> (`self.State Index`) (`self.Current State Index`))
        (set `self.Is Moving Forward` true)
        (`self.TimerCurrentDuration`)
        (`self.InverseDurationCalculation`)
        (bind _returnvalue_2 (`self.SetSpeed` (`KismetMathLibrary.Lerp` (`self.Initial Speed`) _output_2 (/ (`self.Current Duration`) (`|GetArrayItem` (`self.SpeedsUpDuration`) (+ 1 (`self.Current State Index`))))) _output_2))
        (if _returnvalue_2
          (set `self.Current State Index` (+ 1 (`self.Current State Index`)))
          (goto _label))
        (else
          (set `self.Is Moving Backward` true)
          (`self.TimerCurrentDuration`)
          (`self.InverseDurationCalculation`)
          (bind _returnvalue_3 (`self.SetSpeed` (`KismetMathLibrary.Lerp` (`self.Initial Speed`) _output_3 (/ (`self.Current Duration`) (`|GetArrayItem` (`self.SpeedDownDuration`) (- (`self.Current State Index`) 1)))) _output_3))
          (if _returnvalue_3
            (set `self.Current State Index` (- (`self.Current State Index`) 1))
            (goto _label)))))))

(fn `SMLateralSpeed`
  (bind _max_lateral_speed (`self.Max Lateral Speed`))
  (bind _max_lateral_speed_2 (`self.Max Lateral Speed`))
  (if (or (`self.Is Moving Right`) (`self.Is Moving Left`))
    (bind _returnvalue (`self.BooleanConverter` (`self.Is Moving Right`)))
    (set `self.Current Lateral Speed` (`KismetMathLibrary.FClamp` (+ (`self.Current Lateral Speed`) (* _returnvalue (`GameplayStatics.GetWorldDeltaSeconds`) (`self.Multiplier Lateral Speed`))) (* _max_lateral_speed_2 -1.0) _max_lateral_speed_2))
    (elif (`KismetMathLibrary.NearlyEqual_FloatFloat` (`self.Current Lateral Speed`) 0.0 0.1)
      (set `self.Current Lateral Speed` 0.0)
      (else
        (set `self.Current Lateral Speed` (`KismetMathLibrary.FClamp` (- (`self.Current Lateral Speed`) (* (`GameplayStatics.GetWorldDeltaSeconds`) (`KismetMathLibrary.SignOfFloat` (`self.Current Lateral Speed`)) (/ (`self.Multiplier Lateral Speed`) 2.0))) (* _max_lateral_speed -1.0) _max_lateral_speed))))))

(fn `SMVerticalSpeed`
  (bind _max_vertical_speed (`self.Max Vertical Speed`))
  (bind _max_vertical_speed_2 (`self.Max Vertical Speed`))
  (if (or (`self.Is Moving Up`) (`self.Is Moving Down`))
    (bind _returnvalue (`self.BooleanConverter` (`self.Is Moving Up`)))
    (set `self.Current Vertical Speed` (`KismetMathLibrary.FClamp` (+ (`self.Current Vertical Speed`) (* _returnvalue (`GameplayStatics.GetWorldDeltaSeconds`) (`self.Multiplier Vertical Speed`))) (* _max_vertical_speed -1.0) _max_vertical_speed))
    (elif (`KismetMathLibrary.NearlyEqual_FloatFloat` (`self.Current Vertical Speed`) 0.0 0.1)
      (set `self.Current Vertical Speed` 0.0)
      (else
        (set `self.Current Vertical Speed` (`KismetMathLibrary.FClamp` (- (`self.Current Vertical Speed`) (* (`GameplayStatics.GetWorldDeltaSeconds`) (`KismetMathLibrary.SignOfFloat` (`self.Current Vertical Speed`)) (/ (`self.Multiplier Vertical Speed`) 2.0))) (* _max_vertical_speed_2 -1.0) _max_vertical_speed_2))))))

(fn `TimerCurrentDuration`
  (set `self.Current Duration` (+ (`self.Current Duration`) (`GameplayStatics.GetWorldDeltaSeconds`))))

(fn `UserConstructionScript`)