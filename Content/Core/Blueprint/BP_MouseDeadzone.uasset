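; BP_MouseDeadzone checks whether the mouse cursor lies outside a dead zone, gating yaw and pitch separately.
; GetViewportMousePosition sets CanYaw and CanPitch by comparing the X and Y values from GetMousePositionIn2D against DeadZone.
; That helper contains math for absolute cursor offset from viewport center, with a fixed vertical correction, though its output wiring is not shown.
; The event graph holds only disabled stubs.
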(fn `Get Viewport Mouse Position`
  (bind _deadzone (`self.DeadZone`))
  (bind (_locationx _locationy) (`PlayerController.GetMousePosition` (`GameplayStatics.GetPlayerController` 0)))
  (bind (_returnvalue_x _returnvalue_y) (`KismetMathLibrary.BreakVector2D` (/ (`WidgetLayoutLibrary.GetViewportSize`) 2.0)))
  (bind (_returnvalue_x_2 _returnvalue_y_2) (`KismetMathLibrary.BreakVector2D` (`KismetMathLibrary.GetAbs2D` (`KismetMathLibrary.MakeVector2D` (- _locationx _returnvalue_x) (+ (- _returnvalue_y _locationy) 28.0)))))
  (set `self.Can Yaw` (> _returnvalue_x_2 _deadzone))
  (set `self.Can Pitch` (> _returnvalue_y_2 _deadzone)))