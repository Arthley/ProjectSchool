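; Rotation component that turns turn, pitch and roll flags into smoothed per-axis speeds, published each Tick as FinalRotator without applying it.
; Active flags accelerate speeds within clamped limits, with a boolean-to-sign helper setting direction.
; Without input, speeds decay at half that rate and snap to zero.
; For players, normalized yaw speed drives a WB_HUD_Turn slider, re-created when turning and removed once yaw settles.
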(event `self.ReceiveBeginPlay`
  (if (`self.Is Player`)
    (bind _returnvalue (`|CreateWidget` "/Game/Core/Blueprint/Widget/WB_HUD_Turn.WB_HUD_Turn_C" (`GameplayStatics.GetPlayerController` 0)))
    (bind _output_get (set `self.HUD Turn` _returnvalue))
    (`UserWidget.AddToViewport` _output_get 0)))

(event `self.ReceiveTick`
  (params (DeltaSeconds :type "Float (single-precision)"))
  (`self.YawSpeed`)
  (`self.PitchSpeed`)
  (`self.RollSpeed`)
  (set `self.Final Rotator` (`KismetMathLibrary.MakeRotator` (`self.Current Roll Speed`) (`self.Current Pitch Speed`) (`self.Current Yaw Speed`))))

(fn `BooleanConverter`
  (params (Boolean :type Boolean))
  (returns (ReturnValue :type "Float (double-precision)"))
  (return (- (* (+ (`KismetMathLibrary.Conv_BoolToDouble` Boolean) 1.0) 2.0) 3.0)))

(fn `PitchSpeed`
  (bind _max_pitch_speed (`self.Max Pitch Speed`))
  (bind _max_pitch_speed_2 (`self.Max Pitch Speed`))
  (if (or (`self.Is Turning Up`) (`self.Is Turning Down`))
    (bind _returnvalue (`self.BooleanConverter` (`self.Is Turning Up`)))
    (set `self.Current Pitch Speed` (`KismetMathLibrary.FClamp` (+ (`self.Current Pitch Speed`) (* (`GameplayStatics.GetWorldDeltaSeconds`) _returnvalue 0.03)) (* _max_pitch_speed -1.0) _max_pitch_speed))
    (elif (`KismetMathLibrary.NearlyEqual_FloatFloat` (`self.Current Pitch Speed`))
      (set `self.Current Pitch Speed` 0.0)
      (else
        (set `self.Current Pitch Speed` (`KismetMathLibrary.FClamp` (- (`self.Current Pitch Speed`) (* (`GameplayStatics.GetWorldDeltaSeconds`) (`KismetMathLibrary.SignOfFloat` (`self.Current Pitch Speed`)) 0.015)) (* _max_pitch_speed_2 -1.0) _max_pitch_speed_2))))))

(fn `RollSpeed`
  (bind _max_roll_speed (`self.Max Roll Speed`))
  (bind _max_roll_speed_2 (`self.Max Roll Speed`))
  (if (or (`self.Is Rolling Right`) (`self.Is Rolling Left`))
    (bind _returnvalue (`self.BooleanConverter` (`self.Is Rolling Right`)))
    (set `self.Current Roll Speed` (`KismetMathLibrary.FClamp` (+ (`self.Current Roll Speed`) (* (`GameplayStatics.GetWorldDeltaSeconds`) _returnvalue 0.03)) (* _max_roll_speed -1.0) _max_roll_speed))
    (elif (`KismetMathLibrary.NearlyEqual_FloatFloat` (`self.Current Roll Speed`))
      (set `self.Current Roll Speed` 0.0)
      (else
        (set `self.Current Roll Speed` (`KismetMathLibrary.FClamp` (- (`self.Current Roll Speed`) (* (`GameplayStatics.GetWorldDeltaSeconds`) (`KismetMathLibrary.SignOfFloat` (`self.Current Roll Speed`)) 0.015)) (* _max_roll_speed_2 -1.0) _max_roll_speed_2))))))

(fn `YawSpeed`
  (bind _max_yaw_speed (`self.Max Yaw Speed`))
  (bind _max_yaw_speed_2 (`self.Max Yaw Speed`))
  (if (`self.Is Player`)
    (set `/Game/Core/Blueprint/Widget/WB_HUD_Turn.TurnSpeed` (+ (/ (`self.Current Yaw Speed`) (* (`self.Max Yaw Speed`) 2.0)) 0.5) (`self.HUD Turn`)))
  (if (or (`self.Is Turning Left`) (`self.Is Turning Right`))
    (bind _returnvalue (`self.BooleanConverter` (`self.Is Turning Right`)))
    (set `self.Current Yaw Speed` (`KismetMathLibrary.FClamp` (+ (`self.Current Yaw Speed`) (* (`GameplayStatics.GetWorldDeltaSeconds`) _returnvalue 0.03)) (* _max_yaw_speed -1.0) _max_yaw_speed))
    (if (`Widget.IsVisible` (`self.HUD Turn`))
      _
      (elif (`self.Is Player`)
        (bind _returnvalue_2 (`|CreateWidget` "/Game/Core/Blueprint/Widget/WB_HUD_Turn.WB_HUD_Turn_C" (`GameplayStatics.GetPlayerController` 0)))
        (bind _output_get (set `self.HUD Turn` _returnvalue_2))
        (`UserWidget.AddToViewport` _output_get 0)))
    (elif (`KismetMathLibrary.NearlyEqual_FloatFloat` (`self.Current Yaw Speed`) 0.0 0.001)
      (set `self.Current Yaw Speed` 0.0)
      (if (`self.Is Player`)
        (bind _foundwidgets (`WidgetBlueprintLibrary.GetAllWidgetsOfClass` "/Game/Core/Blueprint/Widget/WB_HUD_Turn.WB_HUD_Turn_C"))
        (`Widget.RemoveFromParent` _foundwidgets))
      (else
        (set `self.Current Yaw Speed` (`KismetMathLibrary.FClamp` (- (`self.Current Yaw Speed`) (* (`GameplayStatics.GetWorldDeltaSeconds`) (`KismetMathLibrary.SignOfFloat` (`self.Current Yaw Speed`)) 0.015)) (* _max_yaw_speed_2 -1.0) _max_yaw_speed_2))))))