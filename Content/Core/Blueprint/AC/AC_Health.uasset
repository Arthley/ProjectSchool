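; Health component for spaceships that tracks damage, scores hits and destroys the owning ship at zero health.
; TakeDamage clamps health, then subtracts hit points from BP_Score for a player owner or adds them otherwise.
; Player health updates the HUD as a fraction of max, while death awards kill points for any owner and spawns a Niagara explosion.
; A debug L key applies test damage.
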(event EventBeginPlay
  (Variables|Default|SetHealth (Variables|Default|GetMaxHealth))
  (bind _asbp_space_ship_player (Utilities|Casting|CastToBP_SpaceShipPlayer (Components|GetOwner)))
  (Utilities|FlowControl|Delay 0.2)
  (CallFunction|UpdateHUDHP _asbp_space_ship_player))

(event Input|KeyboardEvents|DebugKeyL
  (params (Key :type Key%20Structure) (ActionValue :type Input%20Action%20Value%20Structure))
  (:Pressed
    (CallFunction|TakeDamage 50)))

(fn TakeDamage
  (params (Damage :type Integer))
  (Variables|Default|SetHealth (Math|Integer|Clamp(Integer) (- (Variables|Default|GetHealth) Damage) 0 (Variables|Default|GetMaxHealth)))
  (Utilities|Casting|CastToBP_SpaceShipPlayer (Components|GetOwner)
    (:then
      (bind _returnvalue (Actor|GetActorOfClass "/Game/Core/Blueprint/Score/BP_Score.BP_Score_C"))
      (Default|AddPointsforShipHit _returnvalue (* (Variables|Default|GetPoints%20for%20Hit) -1))
      (CallFunction|UpdateHUDHP))
    (:CastFailed
      (bind _returnvalue_2 (Actor|GetActorOfClass "/Game/Core/Blueprint/Score/BP_Score.BP_Score_C"))
      (Default|AddPointsforShipHit _returnvalue_2 (Variables|Default|GetPoints%20for%20Hit))))
  (Development|PrintString (Utilities|String|ToString(Integer) (Variables|Default|GetHealth)))
  (CallFunction|DestroyShip))

(fn DestroyShip
  (if (== (Variables|Default|GetHealth) 0.0)
    (bind _asbp_space_ship_base (Utilities|Casting|CastToBP_SpaceShipBase (Components|GetOwner)))
    (bind _returnvalue (Actor|GetActorOfClass "/Game/Core/Blueprint/Score/BP_Score.BP_Score_C"))
    (Default|AddPointsforShipDextroyed _returnvalue (Variables|Default|GetPoints%20for%20Kill))
    (Niagara|SpawnSystematLocation "/Game/Core/Blueprint/SpaceShip/Enemy/NS_ExplosionEnemy.NS_ExplosionEnemy" (Transformation|GetActorLocation _asbp_space_ship_base))
    (Actor|DestroyActor _asbp_space_ship_base)))

(fn UpdateHUDHP
  (params (SpaceShipPlayer :type BP%20Space%20Ship%20Player%20Object%20Reference))
  (Variables|/Game/Core/Blueprint/Widget/WB_HUD_Core.WB_HUD_Core_C|SetCHealthPoint (Variables|/Game/Core/Blueprint/SpaceShip/Player/BP_SpaceShipPlayer.BP_SpaceShipPlayer_C|GetHUD%20Core SpaceShipPlayer) (/ (Variables|Default|GetHealth) (Variables|Default|GetMaxHealth))))