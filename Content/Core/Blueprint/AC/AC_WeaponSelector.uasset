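; Actor component that cycles the owning spaceship's active weapon to the next one in its list.
; SelectWeapon casts the owner to BP_SpaceShipBase, finds WeaponCurrent in WeaponClass and advances it, wrapping to the first entry after the last.
; It then calls UpdateCurrentWeapons on the ship to apply the change.
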(fn `Select Weapon`
  (bind _asbp_space_ship_base (cast `/Game/Core/Blueprint/SpaceShip/BP_SpaceShipBase` (`self.GetOwner`)))
  (bind _weapon_class (`/Game/Core/Blueprint/SpaceShip/BP_SpaceShipBase.Weapon Class` _asbp_space_ship_base))
  (bind _returnvalue (+ (`KismetArrayLibrary.Array_Find` _weapon_class (`/Game/Core/Blueprint/SpaceShip/BP_SpaceShipBase.Weapon Current` _asbp_space_ship_base)) 1))
  (if (== (`KismetArrayLibrary.Array_Length` _weapon_class) _returnvalue)
    (set `/Game/Core/Blueprint/SpaceShip/BP_SpaceShipBase.Weapon Current` (`|GetArrayItem` _weapon_class) _asbp_space_ship_base)
    (else
      (set `/Game/Core/Blueprint/SpaceShip/BP_SpaceShipBase.Weapon Current` (`|GetArrayItem` _weapon_class _returnvalue) _asbp_space_ship_base)))
  (`/Game/Core/Blueprint/SpaceShip/BP_SpaceShipBase.Update Current Weapons` _asbp_space_ship_base))