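; AC_LockOn is an actor component that manages target lock-on for the player spaceship.
; LockOnTarget stores a target if none is locked and shows its lock-on and prediction aim sprites.
; Tick tracks the target's world location, and IA_Unlock hides the sprites and clears the locked flag.
; Unlocking or an invalid target also resets the ship's aim line prediction component.
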(event `self.ReceiveTick`
  (params (DeltaSeconds :type "Float (single-precision)"))
  (bind _lock_target (`self.Lock Target`)
    (:`then`
      (set `self.Target Location` (`SceneComponent.K2_GetComponentLocation` (`/Game/Core/Blueprint/SpaceShip/BP_SpaceshipBase.DefaultSceneRoot` _lock_target))))
    (:`else`
      (set `self.Is Target Locked` false)
      (`self.ResetAimLinePredictionParameters`))))

(event `EnhancedInput|/Game/Core/Blueprint/Input/Inputs/IA_Unlock`
  (params (ActionValue :type Boolean) (ElapsedSeconds :type "Float (double-precision)") (TriggeredSeconds :type "Float (double-precision)") (InputAction :type "InputAction Object Reference" :default "/Game/Core/Blueprint/Input/Inputs/IA_Unlock.IA_Unlock"))
  (:`Started`
    (bind _lock_target (`self.Lock Target`)
      (:`then`
        (set `self.Is Target Locked` false)
        (`SceneComponent.SetHiddenInGame` (`/Game/Core/Blueprint/SpaceShip/Enemy/BP_TestEnemy.Lock On Sprite` _lock_target) true false)
        (`SceneComponent.SetHiddenInGame` (`/Game/Core/Blueprint/SpaceShip/Enemy/BP_TestEnemy.Prediction Aim Sprite` _lock_target) true false)
        (`self.ResetAimLinePredictionParameters`))
      (:`else`))))

(fn `LockOnTarget`
  (params (`Lock to Target` :type "/Game/Core/Blueprint/SpaceShip/Enemy/BP_TestEnemy Object Reference"))
  (if (not (`self.Is Target Locked`))
    (set `self.Is Target Locked` true)
    (bind _output_get (set `self.Lock Target` `Lock to Target`))
    (`SceneComponent.SetHiddenInGame` (`/Game/Core/Blueprint/SpaceShip/Enemy/BP_TestEnemy.Lock On Sprite` _output_get) false false)
    (`SceneComponent.SetHiddenInGame` (`/Game/Core/Blueprint/SpaceShip/Enemy/BP_TestEnemy.Prediction Aim Sprite` `Lock to Target`) false false)
    (`KismetSystemLibrary.PrintString` (`KismetSystemLibrary.GetDisplayName` _output_get))))

(fn `ResetAimLinePredictionParameters`
  (bind _asbp_space_ship_player (cast `/Game/Core/Blueprint/SpaceShip/Player/BP_SpaceShipPlayer` (`self.GetOwner`)))
  (`/Game/Core/Blueprint/AC/AC_AimLinePrediction.Reset Parameters` (`/Game/Core/Blueprint/SpaceShip/Player/BP_SpaceShipPlayer.AC_AimLinePrediction` _asbp_space_ship_player)))