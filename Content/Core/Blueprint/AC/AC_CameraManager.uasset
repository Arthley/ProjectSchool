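; Actor component for BP_SpaceShipPlayer that manages spring-arm camera zoom, aim mode and placement.
; Zoom input adjusts a clamped arm length, entering aim mode at minimum; aim input toggles that mode directly.
; Each tick it applies the arm length and lerps the arm toward one of the owner's arrow components.
; When zoomed in, it picks between two turret points by camera distance with a fixed bias, otherwise using a third.
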(event `self.ReceiveBeginPlay`
  (set `self.Camera Positions` (`Actor.K2_GetComponentsByClass` (`self.GetOwner`) "/Script/Engine.ArrowComponent"))
  (bind _asbp_space_ship_player (cast `/Game/Core/Blueprint/SpaceShip/Player/BP_SpaceShipPlayer` (`self.GetOwner`)))
  (set `self.Current Arm Length` (`SpringArmComponent.TargetArmLength` (`/Game/Core/Blueprint/SpaceShip/Player/BP_SpaceShipPlayer.SpringArm` _asbp_space_ship_player))))

(event `self.ReceiveTick`
  (params (DeltaSeconds :type "Float (single-precision)"))
  (bind _asbp_space_ship_player (cast `/Game/Core/Blueprint/SpaceShip/Player/BP_SpaceShipPlayer` (`self.GetOwner`)))
  (bind _springarm (`/Game/Core/Blueprint/SpaceShip/Player/BP_SpaceShipPlayer.SpringArm` _asbp_space_ship_player))
  (`self.Update Arm Length` _springarm)
  (bind _back_camera_is_closer (`self.Calculate Closest Camera Position` _asbp_space_ship_player))
  (`self.Move Camera Between Points` _back_camera_is_closer _springarm))

(event `EnhancedInput|/Game/Core/Blueprint/Input/Inputs/IA_Zoom`
  (params (ActionValue :type "Float (double-precision)") (ElapsedSeconds :type "Float (double-precision)") (TriggeredSeconds :type "Float (double-precision)") (InputAction :type "InputAction Object Reference" :default "/Game/Core/Blueprint/Input/Inputs/IA_Zoom.IA_Zoom"))
  (bind _returnvalue (* ActionValue (`self.Zoom Speed Value`) -1.0))
  (:`Triggered`
    (bind _asbp_space_ship_player (cast `/Game/Core/Blueprint/SpaceShip/Player/BP_SpaceShipPlayer` (`self.GetOwner`)))
    (if (`self.Is Aim Mode`)
      (if (> _returnvalue 0.0)
        (set `self.Current Arm Length` (`self.Min Zoom Value`))
        (set `self.Is Aim Mode` false))
      (else
        (bind _output_get (set `self.Current Arm Length` (`KismetMathLibrary.FClamp` (+ (`SpringArmComponent.TargetArmLength` (`/Game/Core/Blueprint/SpaceShip/Player/BP_SpaceShipPlayer.SpringArm` _asbp_space_ship_player)) _returnvalue) (`self.Min Zoom Value`) (`self.Max Zoom Value`))))
        (set `self.Is Zoom to Turret` (< _output_get (`self.Zoom Camera Threshold`)))
        (if (== _output_get (`self.Min Zoom Value`))
          (set `self.Is Aim Mode` true))))))

(event `EnhancedInput|/Game/Core/Blueprint/Input/Inputs/IA_Aim`
  (params (ActionValue :type Boolean) (ElapsedSeconds :type "Float (double-precision)") (TriggeredSeconds :type "Float (double-precision)") (InputAction :type "InputAction Object Reference" :default "/Game/Core/Blueprint/Input/Inputs/IA_Aim.IA_Aim"))
  (:`Started`
    (if (`self.Is Aim Mode`)
      (set `self.Is Aim Mode` false)
      (set `self.Is Zoom to Turret` false)
      (set `self.Current Arm Length` (`self.Zoom Camera Threshold`))
      (else
        (set `self.Is Aim Mode` true)
        (set `self.Is Zoom to Turret` true)))))

(fn `Calculate Closest Camera Position`
  (params (SpaceShipPlayer :type "/Game/Core/Blueprint/SpaceShip/Player/BP_SpaceShipPlayer Object Reference"))
  (returns (`Back Camera is Closer` :type Boolean))
  (bind _returnvalue (`SceneComponent.K2_GetComponentLocation` (`/Game/Core/Blueprint/SpaceShip/Player/BP_SpaceShipPlayer.Camera` SpaceShipPlayer)))
  (return (>= (`KismetMathLibrary.VSize` (- (`SceneComponent.K2_GetComponentLocation` (`|GetArrayItem` (`self.Camera Positions`) 1)) _returnvalue)) (+ (`KismetMathLibrary.VSize` (- (`SceneComponent.K2_GetComponentLocation` (`|GetArrayItem` (`self.Camera Positions`))) _returnvalue)) 100.0))))

(fn `Move Camera Between Points`
  (params (`Back Camera is Closer` :type Boolean) (`Spring Arm` :type "SpringArmComponent Object Reference"))
  (if (`self.Is Zoom to Turret`)
    (if `Back Camera is Closer`
      (set `self.Camera Index` 0)
      (else
        (set `self.Camera Index` 1)))
    (else
      (set `self.Camera Index` 2)))
  (`SceneComponent.K2_SetRelativeLocation` `Spring Arm` (`KismetMathLibrary.VLerp` (`SceneComponent.RelativeLocation` `Spring Arm`) (`SceneComponent.RelativeLocation` (`|GetArrayItem` (`self.Camera Positions`) (`self.Camera Index`))) (* (`GameplayStatics.GetWorldDeltaSeconds`) (`self.Camera Movement Speed`))) false false))

(fn `Update Arm Length`
  (params (`Spring Arm` :type "SpringArmComponent Object Reference"))
  (if (`self.Is Aim Mode`)
    (set `SpringArmComponent.TargetArmLength` (`self.Aim Mode Arm Length`) `Spring Arm`)
    (else
      (set `SpringArmComponent.TargetArmLength` (`self.Current Arm Length`) `Spring Arm`))))