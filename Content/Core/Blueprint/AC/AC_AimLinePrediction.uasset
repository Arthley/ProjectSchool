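; Actor component for spaceships that predicts where to aim to hit the locked-on target.
; Each tick it updates a running average frame time, clearable through ResetParameters, and leads the target along its forward vector.
; The lead scales target speed by distance over the first weapon's bullet speed, with bullet speed divided by that average frame time.
; The result is stored as FinalPredictionPoint; player ships also move the enemy target's prediction sprite there.
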(event `self.ReceiveTick`
  (params (DeltaSeconds :type "Float (single-precision)"))
  (`self.Calculate Mean Time`)
  (`self.Find Distance from Target`))

(fn `Calculate Mean Time`
  (set `self.Total Time` (+ (`GameplayStatics.GetWorldDeltaSeconds`) (`self.Total Time`)))
  (set `self.Mean` (+ (`self.Mean`) 1))
  (set `self.Mean Time` (/ (`self.Total Time`) (`self.Mean`))))

(fn `Find Distance from Target`
  (bind _asbp_space_ship_base (cast `/Game/Core/Blueprint/SpaceShip/BP_SpaceShipBase` (`self.GetOwner`)))
  (bind _lock_target (`/Game/Core/Blueprint/AC/AC_LockOn.Lock Target` (`/Game/Core/Blueprint/SpaceShip/BP_SpaceShipBase.AC_LockOn` _asbp_space_ship_base)))
  (`/Engine/EditorBlueprintResources/StandardMacros.IsValid` _lock_target
    (:`Is Valid`
      (cast `/Game/Core/Blueprint/SpaceShip/Player/BP_SpaceShipPlayer` _asbp_space_ship_base
        (:`then`
          (bind _asbp_space_ship_enemy (cast `/Game/Core/Blueprint/SpaceShip/Enemy/BP_SpaceShipEnemy` _lock_target))
          (bind _returnvalue (+ (`Actor.K2_GetActorLocation` _lock_target) (* (`Actor.GetActorForwardVector` _lock_target) (`/Game/Core/Blueprint/SpaceShip/BP_SpaceShipBase.Current Speed` _lock_target) (/ (`KismetMathLibrary.VSize` (- (`Actor.K2_GetActorLocation` _lock_target) (`Actor.K2_GetActorLocation` _asbp_space_ship_base))) (/ (`/Game/Core/Blueprint/Turret/Player/BP_TurretPlayer.Bullet Speed` (`|GetArrayItem` (`/Game/Core/Blueprint/SpaceShip/BP_SpaceShipBase.Current Weapons` _asbp_space_ship_base))) (`self.Mean Time`))))))
          (`SceneComponent.K2_SetWorldLocation` (`/Game/Core/Blueprint/SpaceShip/Enemy/BP_SpaceShipEnemy.Prediction Aim Sprite` _asbp_space_ship_enemy) _returnvalue false false))
        (:`CastFailed`
          _))
      (set `self.Final Prediction Point` _returnvalue))))

(fn `Reset Parameters`
  (set `self.Mean` 0)
  (set `self.Total Time` 0.0))