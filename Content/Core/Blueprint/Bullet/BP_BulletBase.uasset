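; Base bullet actor that moves along its Direction by Speed every tick, without sweeping or delta-time scaling.
; SetBulletDirection randomly picks inner or outer spread by comparing a random float to AlphaPrecision, then replaces Direction with the Dispertion result.
; Dispertion projects the normalized direction 1000 units out, adds per-axis random spread and renormalizes.
; Outer shots also add the inner spread as a fixed positive offset on every axis.
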(event `self.ReceiveTick`
  (params (DeltaSeconds :type "Float (single-precision)"))
  (`self.K2_AddActorWorldOffset` (* (`self.Direction`) (`self.Speed`))))

(fn `Dispertion`
  (params (`Spread Value` :type "Float (double-precision)") (`Is Outer` :type Boolean))
  (returns (ReturnValue :type "Vector Structure"))
  (bind (_random_x _random_y _random_z) (`self.Random Spread` `Spread Value`))
  (bind (_random_x_2 _random_y_2 _random_z_2) (`self.Random Spread` `Spread Value`))
  (bind (_returnvalue_x _returnvalue_y _returnvalue_z) (`KismetMathLibrary.BreakVector` (* (`KismetMathLibrary.Normal` (`self.Direction`)) 1000.0)))
  (bind (_returnvalue_x_2 _returnvalue_y_2 _returnvalue_z_2) (`KismetMathLibrary.BreakVector` (* (`KismetMathLibrary.Normal` (`self.Direction`)) 1000.0)))
  (if `Is Outer`
    (return (`KismetMathLibrary.Normal` (`KismetMathLibrary.MakeVector` (+ _returnvalue_x_2 _random_x (`self.Inner Spread at 1000m`)) (+ _returnvalue_y_2 _random_y (`self.Inner Spread at 1000m`)) (+ _returnvalue_z_2 _random_z (`self.Inner Spread at 1000m`)))))
    (else
      (return (`KismetMathLibrary.Normal` (`KismetMathLibrary.MakeVector` (+ _random_x_2 _returnvalue_x) (+ _random_y_2 _returnvalue_y) (+ _random_z_2 _returnvalue_z)))))))

(fn `Set Bullet Direction`
  (bind _output_get (set `self.Is Outer` (> (`KismetMathLibrary.RandomFloat`) (`self.Alpha Precision`))))
  (if _output_get
    (bind _returnvalue (`self.Dispertion` (`self.Outer Spread at 1000m`) _output_get))
    (set `self.Direction` _returnvalue)
    (else
      (bind _returnvalue_2 (`self.Dispertion` (`self.Inner Spread at 1000m`) _output_get))
      (set `self.Direction` _returnvalue_2))))

(fn `UserConstructionScript`)