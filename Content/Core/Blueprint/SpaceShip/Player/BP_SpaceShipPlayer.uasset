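; Player-controlled spaceship that adds Enhanced Input and the core HUD, with stepped speed levels and engine sounds.
; Input sets movement and ACRotator flags, with a toggle between rotating and moving modes.
; Each tick updates speed sliders, scales FOV with speed and line-traces for an aim point fed to all turrets.
; Hitting a BP_TestEnemy triggers ACLockOn; while locked, trace distance follows the ACAimLinePrediction point.
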(event `self.ReceiveBeginPlay`
  ;[0.8871 0.5121 1] Add Input and HUD
  (`parent.ReceiveBeginPlay`)
  (bind _asplayer_controller (cast `PlayerController` (`self.GetController`)))
  (`/Engine/EditorBlueprintResources/StandardMacros.IsValid` _asplayer_controller
    (:`Is Valid`
      (`EnhancedInputSubsystemInterface.AddMappingContext` (pcsubsystem `EnhancedInputLocalPlayerSubsystem` _asplayer_controller) "/Game/Core/Blueprint/Input/IMC_SpaceShip2D.IMC_SpaceShip2D" 0 (struct))
      (bind _returnvalue (`|CreateWidget` "/Game/Core/Blueprint/Widget/WB_HUD_Core.WB_HUD_Core_C" (`GameplayStatics.GetPlayerController` 0)))
      (bind _output_get (set `self.HUD Core` _returnvalue))
      (`UserWidget.AddToViewport` _output_get 0)
      (`GameplayStatics.PlaySound2D` "/Game/Core/Sound/SFX/SFX_StarshipStartupSound.SFX_StarshipStartupSound" 1.0 1.0 0.0 null null)
      (`AudioComponent.SetSound` (`self.AudioSource`) "/Game/Core/Sound/SFX/SFX_StarshipEngine.SFX_StarshipEngine"))))

(event `self.ReceiveTick`
  (params (DeltaSeconds :type "Float (single-precision)"))
  ;[1 0.1941 0.385] Update Movement
  (`parent.ReceiveTick` DeltaSeconds)
  ;[1 0.383 0.5032] Update HUD
  (`self.Update HUD Speed Slider`)
  ;[0.2834 0.3136 1] Update FOV
  (`self.Update FOV`)
  ;[0.5383 0.4202 1] Targeting System
  (`self.Calculate Distance toTarget`)
  (for _array_element (`self.Turrets`)
    (set `/Game/Core/Blueprint/Turret/Player/BP_TurretPlayer.Hit Location` (`self.Main Hit Location`) _array_element)))

(event `EnhancedInput|/Game/Core/Blueprint/Input/Inputs/IA_SpeedUp`
  (params (ActionValue :type Boolean) (ElapsedSeconds :type "Float (double-precision)") (TriggeredSeconds :type "Float (double-precision)") (InputAction :type "InputAction Object Reference" :default "/Game/Core/Blueprint/Input/Inputs/IA_SpeedUp.IA_SpeedUp"))
  (bind _state_index (`self.State Index`))
  (bind _returnvalue (- (`KismetArrayLibrary.Array_Length` (`self.Speeds`)) 1))
  ;[1 1 1] Input
  (:`Started`
    (if (!= _state_index _returnvalue)
      (bind _output_get (set `self.State Index` (`KismetMathLibrary.Clamp` (+ _state_index 1) 0 _returnvalue)))
      (`GameplayStatics.PlaySound2D` "/Game/Core/Sound/SFX/SFX_StarshipChangeSpeed.SFX_StarshipChangeSpeed" 1.4 (+ (* _output_get 0.05) 0.8) 0.0 null null))))

(event `EnhancedInput|/Game/Core/Blueprint/Input/Inputs/IA_TurnLeft`
  (params (ActionValue :type Boolean) (ElapsedSeconds :type "Float (double-precision)") (TriggeredSeconds :type "Float (double-precision)") (InputAction :type "InputAction Object Reference" :default "/Game/Core/Blueprint/Input/Inputs/IA_TurnLeft.IA_TurnLeft"))
  (bind _ac_rotator (`self.AC_Rotator`))
  ;[1 1 1] Input
  (:`Triggered`
    (if (not (`/Game/Core/Blueprint/AC/AC_Rotator.Is Turning Right` _ac_rotator))
      (set `/Game/Core/Blueprint/AC/AC_Rotator.Is Turning Left` true _ac_rotator)))
  (:`Completed`
    (set `/Game/Core/Blueprint/AC/AC_Rotator.Is Turning Left` false _ac_rotator)))

(event `EnhancedInput|/Game/Core/Blueprint/Input/Inputs/IA_MoveLeft`
  (params (ActionValue :type Boolean) (ElapsedSeconds :type "Float (double-precision)") (TriggeredSeconds :type "Float (double-precision)") (InputAction :type "InputAction Object Reference" :default "/Game/Core/Blueprint/Input/Inputs/IA_MoveLeft.IA_MoveLeft"))
  ;[1 1 1] Input
  (:`Triggered`
    (if (not (`self.Is Moving Right`))
      (set `self.Is Moving Left` true)))
  (:`Completed`
    (set `self.Is Moving Left` false)))

(event `EnhancedInput|/Game/Core/Blueprint/Input/Inputs/IA_TurnRight`
  (params (ActionValue :type Boolean) (ElapsedSeconds :type "Float (double-precision)") (TriggeredSeconds :type "Float (double-precision)") (InputAction :type "InputAction Object Reference" :default "/Game/Core/Blueprint/Input/Inputs/IA_TurnRight.IA_TurnRight"))
  (bind _ac_rotator (`self.AC_Rotator`))
  ;[1 1 1] Input
  (:`Triggered`
    (if (not (`/Game/Core/Blueprint/AC/AC_Rotator.Is Turning Left` _ac_rotator))
      (set `/Game/Core/Blueprint/AC/AC_Rotator.Is Turning Right` true _ac_rotator)))
  (:`Completed`
    (set `/Game/Core/Blueprint/AC/AC_Rotator.Is Turning Right` false _ac_rotator)))

(event `EnhancedInput|/Game/Core/Blueprint/Input/Inputs/IA_MoveRight`
  (params (ActionValue :type Boolean) (ElapsedSeconds :type "Float (double-precision)") (TriggeredSeconds :type "Float (double-precision)") (InputAction :type "InputAction Object Reference" :default "/Game/Core/Blueprint/Input/Inputs/IA_MoveRight.IA_MoveRight"))
  ;[1 1 1] Input
  (:`Triggered`
    (if (not (`self.Is Moving Left`))
      (set `self.Is Moving Right` true)))
  (:`Completed`
    (set `self.Is Moving Right` false)))

(event `EnhancedInput|/Game/Core/Blueprint/Input/Inputs/IA_SpeedDown`
  (params (ActionValue :type Boolean) (ElapsedSeconds :type "Float (double-precision)") (TriggeredSeconds :type "Float (double-precision)") (InputAction :type "InputAction Object Reference" :default "/Game/Core/Blueprint/Input/Inputs/IA_SpeedDown.IA_SpeedDown"))
  (bind _state_index (`self.State Index`))
  ;[1 1 1] Input
  (:`Started`
    (if (!= 0 _state_index)
      (bind _output_get (set `self.State Index` (`KismetMathLibrary.Clamp` (- _state_index 1) 0 (- (`KismetArrayLibrary.Array_Length` (`self.Speeds`)) 1))))
      (`GameplayStatics.PlaySound2D` "/Game/Core/Sound/SFX/SFX_StarshipChangeSpeed.SFX_StarshipChangeSpeed" 1.4 (+ (* _output_get 0.05) 0.8) 0.0 null null))))

(event `EnhancedInput|/Game/Core/Blueprint/Input/Inputs/IA_TurnUp`
  (params (ActionValue :type Boolean) (ElapsedSeconds :type "Float (double-precision)") (TriggeredSeconds :type "Float (double-precision)") (InputAction :type "InputAction Object Reference" :default "/Game/Core/Blueprint/Input/Inputs/IA_TurnUp.IA_TurnUp"))
  (bind _ac_rotator (`self.AC_Rotator`))
  ;[1 1 1] Input
  (:`Triggered`
    (if (not (`/Game/Core/Blueprint/AC/AC_Rotator.Is Turning Down` _ac_rotator))
      (set `/Game/Core/Blueprint/AC/AC_Rotator.Is Turning Up` true _ac_rotator)))
  (:`Completed`
    (set `/Game/Core/Blueprint/AC/AC_Rotator.Is Turning Up` false _ac_rotator)))

(event `EnhancedInput|/Game/Core/Blueprint/Input/Inputs/IA_MoveUp`
  (params (ActionValue :type Boolean) (ElapsedSeconds :type "Float (double-precision)") (TriggeredSeconds :type "Float (double-precision)") (InputAction :type "InputAction Object Reference" :default "/Game/Core/Blueprint/Input/Inputs/IA_MoveUp.IA_MoveUp"))
  ;[1 1 1] Input
  (:`Triggered`
    (if (not (`self.Is Moving Down`))
      (set `self.Is Moving Up` true)))
  (:`Completed`
    (set `self.Is Moving Up` false)))

(event `EnhancedInput|/Game/Core/Blueprint/Input/Inputs/IA_TurnDown`
  (params (ActionValue :type Boolean) (ElapsedSeconds :type "Float (double-precision)") (TriggeredSeconds :type "Float (double-precision)") (InputAction :type "InputAction Object Reference" :default "/Game/Core/Blueprint/Input/Inputs/IA_TurnDown.IA_TurnDown"))
  (bind _ac_rotator (`self.AC_Rotator`))
  ;[1 1 1] Input
  (:`Triggered`
    (if (not (`/Game/Core/Blueprint/AC/AC_Rotator.Is Turning Up` _ac_rotator))
      (set `/Game/Core/Blueprint/AC/AC_Rotator.Is Turning Down` true _ac_rotator)))
  (:`Completed`
    (set `/Game/Core/Blueprint/AC/AC_Rotator.Is Turning Down` false _ac_rotator)))

(event `EnhancedInput|/Game/Core/Blueprint/Input/Inputs/IA_MoveDown`
  (params (ActionValue :type Boolean) (ElapsedSeconds :type "Float (double-precision)") (TriggeredSeconds :type "Float (double-precision)") (InputAction :type "InputAction Object Reference" :default "/Game/Core/Blueprint/Input/Inputs/IA_MoveDown.IA_MoveDown"))
  ;[1 1 1] Input
  (:`Triggered`
    (if (not (`self.Is Moving Up`))
      (set `self.Is Moving Down` true)))
  (:`Completed`
    (set `self.Is Moving Down` false)))

(event `EnhancedInput|/Game/Core/Blueprint/Input/Inputs/IA_RollLeft`
  (params (ActionValue :type Boolean) (ElapsedSeconds :type "Float (double-precision)") (TriggeredSeconds :type "Float (double-precision)") (InputAction :type "InputAction Object Reference" :default "/Game/Core/Blueprint/Input/Inputs/IA_RollLeft.IA_RollLeft"))
  (bind _ac_rotator (`self.AC_Rotator`))
  ;[1 1 1] Input
  (:`Triggered`
    (if (not (`/Game/Core/Blueprint/AC/AC_Rotator.Is Rolling Right` _ac_rotator))
      (set `/Game/Core/Blueprint/AC/AC_Rotator.Is Rolling Left` true _ac_rotator)))
  (:`Completed`
    (set `/Game/Core/Blueprint/AC/AC_Rotator.Is Rolling Left` false _ac_rotator)))

(event `EnhancedInput|/Game/Core/Blueprint/Input/Inputs/IA_SwitchMode`
  (params (ActionValue :type Boolean) (ElapsedSeconds :type "Float (double-precision)") (TriggeredSeconds :type "Float (double-precision)") (InputAction :type "InputAction Object Reference" :default "/Game/Core/Blueprint/Input/Inputs/IA_SwitchMode.IA_SwitchMode"))
  ;[1 1 1] Input
  (:`Started`
    (`/Engine/EditorBlueprintResources/StandardMacros.FlipFlop`
      (:`A`
        (`self.Deactivate Rotating Mode`))
      (:`B`
        (`self.Activate Rotating Mode`)))))

(event `EnhancedInput|/Game/Core/Blueprint/Input/Inputs/IA_RollRight`
  (params (ActionValue :type Boolean) (ElapsedSeconds :type "Float (double-precision)") (TriggeredSeconds :type "Float (double-precision)") (InputAction :type "InputAction Object Reference" :default "/Game/Core/Blueprint/Input/Inputs/IA_RollRight.IA_RollRight"))
  (bind _ac_rotator (`self.AC_Rotator`))
  ;[1 1 1] Input
  (:`Triggered`
    (if (not (`/Game/Core/Blueprint/AC/AC_Rotator.Is Rolling Left` _ac_rotator))
      (set `/Game/Core/Blueprint/AC/AC_Rotator.Is Rolling Right` true _ac_rotator)))
  (:`Completed`
    (set `/Game/Core/Blueprint/AC/AC_Rotator.Is Rolling Right` false _ac_rotator)))

(event `EnhancedInput|/Game/Core/Blueprint/Input/Inputs/IA_Shoot`
  (params (ActionValue :type Boolean) (ElapsedSeconds :type "Float (double-precision)") (TriggeredSeconds :type "Float (double-precision)") (InputAction :type "InputAction Object Reference" :default "/Game/Core/Blueprint/Input/Inputs/IA_Shoot.IA_Shoot"))
  (bind _turrets (`self.Turrets`))
  ;[1 1 1] Input
  (:`Triggered`
    (for _array_element _turrets
      (set `/Game/Core/Blueprint/Turret/Player/BP_TurretPlayer.Is Firing` true _array_element)))
  (:`Completed`
    (for _array_element_2 _turrets
      (set `/Game/Core/Blueprint/Turret/Player/BP_TurretPlayer.Is Firing` false _array_element_2))))

(fn `Activate Rotating Mode`
  (set `self.Is Rotating Mode` true)
  (set `self.Is Moving Up` false)
  (set `self.Is Moving Down` false)
  (set `self.Is Moving Left` false)
  (set `self.Is Moving Right` false))

(fn `Calculate Distance toTarget`
  (`self.Calculate Target Distance`)
  (bind (_returnvalue _outhit) (`self.Distance to Target`))
  (if _returnvalue
    (bind (_bblockinghit _binitialoverlap _time _distance _location _impactpoint _normal _impactnormal _physmat _hitactor _hitcomponent _hitbonename _bonename _hititem _elementindex _faceindex _tracestart _traceend) (`GameplayStatics.BreakHitResult` _outhit))
    (set `self.Main Hit Location` _impactpoint)
    (bind _asbp_test_enemy (cast `/Game/Core/Blueprint/SpaceShip/Enemy/BP_TestEnemy` _hitactor)
      (:`then`
        (`/Game/Core/Blueprint/AC/AC_LockOn.LockOnTarget` (`self.AC_LockOn`) _asbp_test_enemy)
        (return))
      (:`CastFailed`
        _))
    (else
      (set `self.Main Hit Location` _traceend)))
  (return))

(fn `Calculate Target Distance`
  (if (`/Game/Core/Blueprint/AC/AC_LockOn.Is Target Locked` (`self.AC_LockOn`))
    (set `self.Target Distance` (`KismetMathLibrary.VSize` (- (`/Game/Core/Blueprint/AC/AC_AimLinePrediction.Final Prediction Point` (`self.AC_AimLinePrediction`)) (`self.K2_GetActorLocation`))))
    (else
      (set `self.Target Distance` 100000.0))))

(fn `Deactivate Rotating Mode`
  (bind _ac_rotator (`self.AC_Rotator`))
  (set `self.Is Rotating Mode` false)
  (set `/Game/Core/Blueprint/AC/AC_Rotator.Is Turning Left` false _ac_rotator)
  (set `/Game/Core/Blueprint/AC/AC_Rotator.Is Turning Right` false _ac_rotator)
  (set `/Game/Core/Blueprint/AC/AC_Rotator.Is Turning Down` false _ac_rotator)
  (set `/Game/Core/Blueprint/AC/AC_Rotator.Is Turning Up` false _ac_rotator)
  (set `/Game/Core/Blueprint/AC/AC_Rotator.Is Rolling Left` false _ac_rotator)
  (set `/Game/Core/Blueprint/AC/AC_Rotator.Is Rolling Right` false _ac_rotator))

(fn `Distance to Target`
  (returns (ReturnValue :type Boolean) (OutHit :type "HitResult Structure"))
  (bind _returnvalue (`SceneComponent.K2_GetComponentLocation` (`self.SpringArm`)))
  (bind (_outhit _returnvalue_2) (`KismetSystemLibrary.LineTraceSingle` :`Start` _returnvalue :`End` (+ _returnvalue (* (`KismetMathLibrary.Normal` (- _returnvalue (`SceneComponent.K2_GetComponentLocation` (`self.Camera`)))) (`self.Target Distance`))) :`TraceChannel` "TraceTypeQuery3" :`DrawDebugType` "ForOneFrame" :`DrawTime` 8.0))
  (return _returnvalue_2 _outhit))

(fn `Update FOV`
  (`CameraComponent.SetFieldOfView` (`self.Camera`) (`KismetMathLibrary.FClamp` (+ (* (/ (- (`self.Max FOV`) (`self.Min Fov`)) (`|GetArrayItem` (`self.Speeds`) 5)) (`self.Current Speed`)) (`self.Min Fov`)) (`self.Min Fov`) (`self.Max FOV`)))
  (return))

(fn `Update HUD Speed Slider`
  (bind _speeds (`self.Speeds`))
  (set `/Game/Core/Blueprint/Widget/WB_HUD_Core.TSpeedSlider` (/ (`KismetMathLibrary.Conv_IntToDouble` (`self.State Index`)) 5.0) (`self.HUD Core`))
  (set `/Game/Core/Blueprint/Widget/WB_HUD_Core.CSpeedSlider` (+ (/ (`self.Current Speed`) (- (`|GetArrayItem` _speeds (- (`KismetArrayLibrary.Array_Length` _speeds) 1)) (`|GetArrayItem` _speeds))) 0.2) (`self.HUD Core`)))

(fn `UserConstructionScript`)