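; Base spaceship actor that handles flight movement, links itself to its health component and collects its child player turrets at BeginPlay.
; Each Tick moves it without sweep along mesh forward, up and right axes, and applies the rotator component's rotation.
; Forward speed lerps through indexed gears one step at a time, with timed transitions.
; Vertical and lateral speeds ramp within limits while movement flags are set, then decay at half that rate.
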(event `self.ReceiveBeginPlay`
  (set `/Game/Core/Blueprint/AC/AC_Health.Parent` self (`self.AC_Health`))
  (bind _output_get (set `self.State Index` 1))
  (set `self.Current State Index` _output_get)
  (`self.Add Turret`))

(event `self.ReceiveTick`
  (params (DeltaSeconds :type "Float (single-precision)"))
  ;[1 0.383 0.5032] Movement by step
  (bind _finalspeed (`self.CalculateSpeed` DeltaSeconds))
  (`self.K2_AddActorWorldOffset` _finalspeed)
  (`SceneComponent.K2_AddLocalRotation` (`self.DefaultSceneRoot`) (`/Game/Core/Blueprint/AC/AC_Rotator.Final Rotator` (`self.AC_Rotator`)) false false)
  (`self.SMHorizontalSpeed`)
  (`self.SMLateralSpeed`)
  (`self.SMVerticalSpeed`))

(fn `Add Turret`
  (for _array_element (`self.GetAllChildActors` true)
    (bind _asbp_turret_player (cast `/Game/Core/Blueprint/Turret/Player/BP_TurretPlayer` _array_element))
    (`KismetArrayLibrary.Array_Add` (`self.Turrets`) _asbp_turret_player)))

(fn `BooleanConverter`
  (params (Boolean :type Boolean))
  (returns (ReturnValue :type "Float (double-precision)"))
  (return (- (* (+ (`KismetMathLibrary.Conv_BoolToDouble` Boolean) 1.0) 2.0) 3.0)))

(fn `CalculateSpeed`
  (params (DeltaSeconds :type "Float (single-precision)"))
  (returns (FinalSpeed :type "Vector Structure"))
  (return (* (+ (* (`KismetMathLibrary.Normal` (`SceneComponent.GetForwardVector` (`self.StaticMesh`))) (`self.Current Speed`)) (* (`KismetMathLibrary.Normal` (`SceneComponent.GetUpVector` (`self.StaticMesh`))) (`self.Current Vertical Speed`)) (* (`KismetMathLibrary.Normal` (`SceneComponent.GetRightVector` (`self.StaticMesh`))) (`self.Current Lateral Speed`))) DeltaSeconds)))

(fn `InverseDurationCalculation`
  (set `self.Inverse Duration` (`self.Current Duration`)))

(fn `ResetParametersafterAcceleration`
  (bind _output_get (set `self.Current Speed` (`|GetArrayItem` (`self.Speeds`) (`self.Current State Index`))))
  (set `self.Initial Speed` _output_get)
  (set `self.Current Duration` 0.0)
  (return))

(fn `SetSpeed`
  (params (`Current Speed` :type "Float (double-precision)") (`Speed by Index` :type "Float (double-precision)"))
  (returns (ReturnValue :type Boolean))
  (set `self.Current Speed` `Current Speed`)
  (return (`KismetMathLibrary.NearlyEqual_FloatFloat` `Current Speed` `Speed by Index` 1.0)))

(fn `SMHorizontalSpeed`
  (bind _output (`|GetArrayItem` (`self.Speeds`) (`self.Current State Index`)))
  (bind _output_2 (`|GetArrayItem` (`self.Speeds`) (+ 1 (`self.Current State Index`))))
  (bind _output_3 (`|GetArrayItem` (`self.Speeds`) (- (`self.Current State Index`) 1)))
  (if (== (`self.State Index`) (`self.Current State Index`))
    (if (or (`self.Is Moving Forward`) (`self.Is Moving Backward`))
      (set `self.Current Duration` 0.0)
      (set `self.Is Moving Forward` false)
      (set `self.Is Moving Backward` false))
    (set `self.Initial Speed` (`self.Current Speed`))
    (`self.TimerCurrentDuration`)
    (bind _returnvalue (`self.SetSpeed` (`KismetMathLibrary.Lerp` (`self.Initial Speed`) _output (/ (`self.Current Duration`) (`self.Inverse Duration`))) _output))
    (if _returnvalue
      (`self.ResetParametersafterAcceleration` :!label _label))
    (else
      (if (not (or (`self.Is Moving Forward`) (`self.Is Moving Backward`)))
        (set `self.Current Duration` 0.0))
      (if (> (`self.State Index`) (`self.Current State Index`))
        (set `self.Is Moving Forward` true)
        (`self.TimerCurrentDuration`)
        (`self.InverseDurationCalculation`)
        (bind _returnvalue_2 (`self.SetSpeed` (`KismetMathLibrary.Lerp` (`self.Initial Speed`) _output_2 (/ (`self.Current Duration`) (`|GetArrayItem` (`self.SpeedsUpDuration`) (+ 1 (`self.Current State Index`))))) _output_2))
        (if _returnvalue_2
          (set `self.Current State Index` (+ 1 (`self.Current State Index`)))
          (goto _label))
        (else
          (set `self.Is Moving Backward` true)
          (`self.TimerCurrentDuration`)
          (`self.InverseDurationCalculation`)
          (bind _returnvalue_3 (`self.SetSpeed` (`KismetMathLibrary.Lerp` (`self.Initial Speed`) _output_3 (/ (`self.Current Duration`) (`|GetArrayItem` (`self.SpeedDownDuration`) (- (`self.Current State Index`) 1)))) _output_3))
          (if _returnvalue_3
            (set `self.Current State Index` (- (`self.Current State Index`) 1))
            (goto _label)))))))

(fn `SMLateralSpeed`
  (bind _max_lateral_speed (`self.Max Lateral Speed`))
  (bind _max_lateral_speed_2 (`self.Max Lateral Speed`))
  (if (or (`self.Is Moving Right`) (`self.Is Moving Left`))
    (bind _returnvalue (`self.BooleanConverter` (`self.Is Moving Right`)))
    (set `self.Current Lateral Speed` (`KismetMathLibrary.FClamp` (+ (`self.Current Lateral Speed`) (* _returnvalue (`GameplayStatics.GetWorldDeltaSeconds`) (`self.Multiplier Lateral Speed`))) (* _max_lateral_speed_2 -1.0) _max_lateral_speed_2))
    (elif (`KismetMathLibrary.NearlyEqual_FloatFloat` (`self.Current Lateral Speed`) 0.0 0.1)
      (set `self.Current Lateral Speed` 0.0)
      (else
        (set `self.Current Lateral Speed` (`KismetMathLibrary.FClamp` (- (`self.Current Lateral Speed`) (* (`GameplayStatics.GetWorldDeltaSeconds`) (`KismetMathLibrary.SignOfFloat` (`self.Current Lateral Speed`)) (/ (`self.Multiplier Lateral Speed`) 2.0))) (* _max_lateral_speed -1.0) _max_lateral_speed))))))

(fn `SMVerticalSpeed`
  (bind _max_vertical_speed (`self.Max Vertical Speed`))
  (bind _max_vertical_speed_2 (`self.Max Vertical Speed`))
  (if (or (`self.Is Moving Up`) (`self.Is Moving Down`))
    (bind _returnvalue (`self.BooleanConverter` (`self.Is Moving Up`)))
    (set `self.Current Vertical Speed` (`KismetMathLibrary.FClamp` (+ (`self.Current Vertical Speed`) (* _returnvalue (`GameplayStatics.GetWorldDeltaSeconds`) (`self.Multiplier Vertical Speed`))) (* _max_vertical_speed -1.0) _max_vertical_speed))
    (elif (`KismetMathLibrary.NearlyEqual_FloatFloat` (`self.Current Vertical Speed`) 0.0 0.1)
      (set `self.Current Vertical Speed` 0.0)
      (else
        (set `self.Current Vertical Speed` (`KismetMathLibrary.FClamp` (- (`self.Current Vertical Speed`) (* (`GameplayStatics.GetWorldDeltaSeconds`) (`KismetMathLibrary.SignOfFloat` (`self.Current Vertical Speed`)) (/ (`self.Multiplier Vertical Speed`) 2.0))) (* _max_vertical_speed_2 -1.0) _max_vertical_speed_2))))))

(fn `TimerCurrentDuration`
  (set `self.Current Duration` (+ (`self.Current Duration`) (`GameplayStatics.GetWorldDeltaSeconds`))))

(fn `UserConstructionScript`)