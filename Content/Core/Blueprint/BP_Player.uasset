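; Player spaceship that flies continuously forward and steers toward the mouse cursor.
; Tick moves the actor, then eases its yaw and pitch toward the deprojected cursor direction, each axis gated by the BPMouseDeadzone component.
; Enhanced Input actions adjust speed and roll the Ship component locally, using helper functions driven by hold time.
; A debug line trace along the mouse direction exists but never runs.
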(event `self.ReceiveBeginPlay`
  (bind _asplayer_controller (cast `PlayerController` (`self.GetController`)))
  (`/Engine/EditorBlueprintResources/StandardMacros.IsValid` _asplayer_controller
    (:`Is Valid`
      (`EnhancedInputSubsystemInterface.AddMappingContext` (pcsubsystem `EnhancedInputLocalPlayerSubsystem` _asplayer_controller) "/Game/Core/Blueprint/Input/IMC_Spaceship.IMC_Spaceship" 0 (struct))
      (set `PlayerController.bShowMouseCursor` true (`GameplayStatics.GetPlayerController` 0)))))

(event `self.ReceiveTick`
  (params (DeltaSeconds :type "Float (single-precision)"))
  (bind _bp_mousedeadzone (`self.BP_MouseDeadzone`))
  (bind (_rotation_roll _rotation_pitch _rotation_yaw) (`KismetMathLibrary.BreakRotator` (`self.Rotation`)))
  (bind (_rotation_roll_2 _rotation_pitch_2 _rotation_yaw_2) (`KismetMathLibrary.BreakRotator` (`self.Rotation`)))
  (bind (_worldlocation _worlddirection) (`PlayerController.DeprojectMousePositionToWorld` (`GameplayStatics.GetPlayerController` 0)))
  (bind (_returnvalue_roll _returnvalue_pitch _returnvalue_yaw) (`KismetMathLibrary.BreakRotator` (`KismetMathLibrary.FindLookAtRotation` (`self.K2_GetActorLocation`) (+ _worldlocation (* _worlddirection 5000.0)))))
  (`self.K2_AddActorWorldOffset` (* DeltaSeconds (* (`KismetMathLibrary.Normal` (`SceneComponent.GetForwardVector` (`self.Ship`))) (`self.Speed`))))
  (`/Game/Core/Blueprint/BP_MouseDeadzone.Get Viewport Mouse Position` _bp_mousedeadzone)
  (`|ExecutionSequence`
    (:`then_0`
      (if (`/Game/Core/Blueprint/BP_MouseDeadzone.Can Yaw` _bp_mousedeadzone)
        (set `self.Rotation` (`KismetMathLibrary.MakeRotator` _rotation_roll_2 _rotation_pitch_2 _returnvalue_yaw))
        (else
          (set `self.Rotation` (`KismetMathLibrary.MakeRotator` _rotation_roll_2 _rotation_pitch_2 _rotation_yaw_2)))))
    (:`then_1`
      (if (`/Game/Core/Blueprint/BP_MouseDeadzone.Can Pitch` _bp_mousedeadzone)
        (set `self.Rotation` (`KismetMathLibrary.MakeRotator` _rotation_roll _returnvalue_pitch _rotation_yaw))
        (else
          (set `self.Rotation` (`KismetMathLibrary.MakeRotator` _rotation_roll _rotation_pitch _rotation_yaw)))))
    (:`then_2`
      (`self.K2_SetActorRotation` (`KismetMathLibrary.RInterpTo` (`self.K2_GetActorRotation`) (`self.Rotation`) 0.5 0.05)))))

(event `EnhancedInput|/Game/Core/Blueprint/Input/IA_SpeedUp`
  (params (ActionValue :type Boolean) (ElapsedSeconds :type "Float (double-precision)") (TriggeredSeconds :type "Float (double-precision)") (InputAction :type "InputAction Object Reference" :default "/Game/Core/Blueprint/Input/IA_SpeedUp.IA_SpeedUp"))
  (bind _acceleration (`self.Acceleration`))
  (:`Triggered`
    (set `self.Speed` (`KismetMathLibrary.FClamp` (+ (`self.Speed`) (`KismetMathLibrary.FClamp` (* ElapsedSeconds _acceleration) _acceleration (`self.Max Acceleration`))) (`self.Min Speed`) (`self.Max Speed`)))))

(event `EnhancedInput|/Game/Core/Blueprint/Input/IA_SpeedDown`
  (params (ActionValue :type Boolean) (ElapsedSeconds :type "Float (double-precision)") (TriggeredSeconds :type "Float (double-precision)") (InputAction :type "InputAction Object Reference" :default "/Game/Core/Blueprint/Input/IA_SpeedDown.IA_SpeedDown"))
  (bind _acceleration (`self.Acceleration`))
  (:`Triggered`
    (set `self.Speed` (`KismetMathLibrary.FClamp` (- (`self.Speed`) (`KismetMathLibrary.FClamp` (* ElapsedSeconds _acceleration) _acceleration (`self.Max Acceleration`))) (`self.Min Speed`) (`self.Max Speed`)))))

(event `EnhancedInput|/Game/Core/Blueprint/Input/IA_RollRight`
  (params (ActionValue :type Boolean) (ElapsedSeconds :type "Float (double-precision)") (TriggeredSeconds :type "Float (double-precision)") (InputAction :type "InputAction Object Reference" :default "/Game/Core/Blueprint/Input/IA_RollRight.IA_RollRight"))
  (bind _rotacceleration (`self.RotAcceleration`))
  (bind _rotation_roll (`KismetMathLibrary.BreakRotator` (`self.Rotation`)))
  (:`Triggered`
    (`SceneComponent.K2_AddLocalRotation` (`self.Ship`) (`KismetMathLibrary.MakeRotator` (+ _rotation_roll (`KismetMathLibrary.FClamp` (* ElapsedSeconds _rotacceleration) _rotacceleration (`self.Max RotAcceleration`)))) false false)))

(event `EnhancedInput|/Game/Core/Blueprint/Input/IA_RollLeft`
  (params (ActionValue :type Boolean) (ElapsedSeconds :type "Float (double-precision)") (TriggeredSeconds :type "Float (double-precision)") (InputAction :type "InputAction Object Reference" :default "/Game/Core/Blueprint/Input/IA_RollLeft.IA_RollLeft"))
  (bind _rotacceleration (`self.RotAcceleration`))
  (bind _rotation_roll (`KismetMathLibrary.BreakRotator` (`self.Rotation`)))
  (:`Triggered`
    (`SceneComponent.K2_AddLocalRotation` (`self.Ship`) (`KismetMathLibrary.MakeRotator` (- _rotation_roll (`KismetMathLibrary.FClamp` (* ElapsedSeconds _rotacceleration) _rotacceleration (`self.Max RotAcceleration`)))) false false)))

(fn `UserConstructionScript`)