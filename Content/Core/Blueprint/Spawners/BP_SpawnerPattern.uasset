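; BP_SpawnerPattern drives a group of BP_Spawner child actors, firing a random subset of them in repeated waves.
; BeginPlay gathers its child spawners into SpawnList and looks up BP_Score, though the result is not used.
; Tick runs a DoOnce-gated wave that triggers each spawner by a weighted random roll, then resets after SpawnInterval plus random extra delay.
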(event `self.ReceiveBeginPlay`
  (`GameplayStatics.GetActorOfClass` "/Game/Core/Blueprint/Score/BP_Score.BP_Score_C")
  (for _array_element (`self.GetAllChildActors` true)
    (bind _asbp_spawner (cast `/Game/Core/Blueprint/Spawners/BP_Spawner` _array_element))
    (`KismetArrayLibrary.Array_Add` (`self.Spawn List`) _asbp_spawner)))

(event `self.ReceiveTick`
  (params (DeltaSeconds :type "Float (single-precision)"))
  (`/Engine/EditorBlueprintResources/StandardMacros.DoOnce` false :!label _label
    (:`Completed`
      (for _array_element (`self.Spawn List`)
        (if (>= (`KismetMathLibrary.RandomFloat`) 0.3)
          (`/Game/Core/Blueprint/Spawners/BP_Spawner.Spawner Actor` _array_element)))
      (`KismetSystemLibrary.Delay` (+ (`self.Spawn Interval`) (* (`KismetMathLibrary.RandomFloat`) (`self.Spawn Interval Randomness`))))
      (goto _label :!via `Reset`))))

(fn `UserConstructionScript`)