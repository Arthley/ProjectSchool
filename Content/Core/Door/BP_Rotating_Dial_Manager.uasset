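; Manager for a rotating dial puzzle that checks whether a set of rotators matches its solution.
; CheckSolved compares each rotator's CurrentRotation to the same-index entry in SolveIndex, clearing the Solved flag and stopping at the first mismatch.
; A full match calls CompleteRotators, which swaps the Cube's material to AdvancedFlag.
; A failed check resets Solved to true for the next attempt.
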(event `CheckSolved`
  (for (_array_element _array_index) (`self.Rotators`)
    (if (not (== (`/Game/Core/Door/BP_Rotating_Dial.CurrentRotation` _array_element) (`|GetArrayItem` (`self.SolveIndex`) _array_index)))
      (set `self.Solved` false)
      (break)))
  (if (`self.Solved`)
    (`self.CompleteRotators`)
    (else
      (set `self.Solved` true))))

(fn `CompleteRotators`
  (`PrimitiveComponent.SetMaterial` (`self.Cube`) 0 "/Engine/MaterialTemplates/VertexAnimation/AdvancedFlag.AdvancedFlag"))

(fn `UserConstructionScript`)