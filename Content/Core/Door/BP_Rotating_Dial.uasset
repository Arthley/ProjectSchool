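; Rotating dial actor that turns clockwise by a fixed Rotation step each time its RotateClockwise event is called.
; The event first adds the step to CurrentRotation, wrapping at 360 degrees to track the dial's logical position.
; A Rotate timeline then animates actor yaw from its captured starting value to that value plus the step.
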(event `Rotate Clockwise`
  (bind (_returnvalue_roll _returnvalue_pitch _returnvalue_yaw) (`KismetMathLibrary.BreakRotator` (`self.K2_GetActorRotation`)))
  (bind _startingrotation (`self.StartingRotation`))
  (`self.IncreaseRotationIndex`)
  (set `self.StartingRotation` _returnvalue_yaw)
  (bind (_direction _rotation) (`Timeline|Rotate` :!via `PlayFromStart`)
    (:`Update`
      (`self.K2_SetActorRotation` (`KismetMathLibrary.MakeRotator` 0.0 0.0 (`KismetMathLibrary.Lerp` _startingrotation (+ _startingrotation (`self.Rotation`)) _rotation))))))

(fn `IncreaseRotationIndex`
  (bind _returnvalue (+ (`self.Rotation`) (`self.CurrentRotation`)))
  (if (>= _returnvalue 360.0)
    (set `self.CurrentRotation` (- _returnvalue 360.0))
    (else
      (set `self.CurrentRotation` _returnvalue))))

(fn `UserConstructionScript`)